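; Train hazard actor that repeatedly runs along a straight path and squashes the player's chicken on impact.
; Tick pushes it along local Y by a random step each frame, so its speed jitters and depends on frame rate.
; A looping delay from BeginPlay returns it to its recorded spawn point every eight seconds.
; Mesh hits on a MyChicken set IsDead and flatten the chicken's Z scale.
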(event `self.ReceiveBeginPlay`
  (set `self.SpawnPoint` (`SceneComponent.K2_GetComponentLocation` (`self.DefaultSceneRoot`)))
  (`KismetSystemLibrary.Delay` 8.0 :!label _label)
  (`KismetSystemLibrary.K2_ClearTimer` null)
  (`self.K2_SetActorLocation` (`self.SpawnPoint`))
  (goto _label))

(event `self.ReceiveTick`
  (params (DeltaSeconds :type "Float (single-precision)"))
  (`self.K2_AddActorLocalOffset` (`KismetMathLibrary.MakeVector` 0.0 (`KismetMathLibrary.RandomFloatInRange` 55.0 100.0))))

(event `self.StaticMesh.OnComponentHit`
  (params (HitComponent :type "PrimitiveComponent Object Reference") (OtherActor :type "Actor Object Reference") (OtherComp :type "PrimitiveComponent Object Reference") (NormalImpulse :type "Vector Structure") (Hit :type "HitResult Structure (by ref)"))
  (bind _asmy_chicken (cast `/Game/BluePrints/MyChicken` OtherActor))
  (set `/Game/BluePrints/MyChicken.is Dead` true _asmy_chicken)
  (`SceneComponent.SetRelativeScale3D` (`/Game/BluePrints/MyChicken.chicken` _asmy_chicken) (1.0 1.0 0.1)))

(fn `UserConstructionScript`)