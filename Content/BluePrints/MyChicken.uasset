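; Player chicken character for a Crossy Road-style hopper that creates the HUD and tracks score and coins.
; Directional inputs rotate the mesh, jump and shift the actor one fixed step, gated by a short cooldown and side and rear bounds.
; Tick awards score for forward progress and flags falls as death.
; Death plays train, water or default squash effects once, then restarts the level after a delay.
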(event `self.ReceiveBeginPlay`
  (bind _returnvalue (`|CreateWidget` "/Game/BluePrints/CRHud.CRHud_C" (`GameplayStatics.GetPlayerController` 0)))
  (`UserWidget.AddToViewport` _returnvalue 0))

(event `self.ReceiveTick`
  (params (DeltaSeconds :type "Float (single-precision)"))
  (`self.setscore`)
  (`self.hasfallen`)
  (if (`self.is Dead`)
    (`/Engine/EditorBlueprintResources/StandardMacros.DoOnce` false
      (:`Completed`
        (`self.Death`)
        (`KismetSystemLibrary.Delay` 2.0)
        (`KismetSystemLibrary.ExecuteConsoleCommand` "restartlevel" null)))))

(event `InputAxis|Forward_Backward`
  (params (AxisValue :type "Float (single-precision)"))
  ;[1 1 1] movement
)

(event `InputAxis|Left_Right`
  (params (AxisValue :type "Float (single-precision)"))
  ;[1 1 1] movement
)

(event `InputAction|Left`
  (params (Key :type "Key Structure"))
  (bind (_returnvalue_x _returnvalue_y _returnvalue_z) (`KismetMathLibrary.BreakVector` (`self.K2_GetActorLocation`)))
  ;[1 1 1] movement
  (:`Pressed`
    (if (not (`self.is Dead`))
      (bind _newparam (`self.isMovableLeft`))
      (if _newparam
        (if (not (`self.BoolJump`))
          (`SceneComponent.K2_SetRelativeRotation` (`self.Mesh`) (struct :`Yaw` 270.0) false false)
          (`self.Jump`)
          (set `self.BoolJump` true)
          (`GameplayStatics.PlaySoundAtLocation` "/Game/Sounds/jump1.jump1" (0.0 0.0 0.0) (struct) 1.0 1.0 0.0 null null null)
          (`self.K2_SetActorRelativeLocation` (`KismetMathLibrary.MakeVector` _returnvalue_x (+ _returnvalue_y -150.0) _returnvalue_z))
          (`KismetSystemLibrary.Delay` 0.5)
          (set `self.BoolJump` false))))))

(event `InputAction|Right`
  (params (Key :type "Key Structure"))
  (bind (_returnvalue_x _returnvalue_y _returnvalue_z) (`KismetMathLibrary.BreakVector` (`self.K2_GetActorLocation`)))
  ;[1 1 1] movement
  (:`Pressed`
    (if (not (`self.is Dead`))
      (bind _newparam (`self.isMovableRIght`))
      (if _newparam
        (if (not (`self.BoolJump`))
          (`SceneComponent.K2_SetRelativeRotation` (`self.Mesh`) (struct :`Yaw` 90.0) false false)
          (`self.Jump`)
          (set `self.BoolJump` true)
          (`GameplayStatics.PlaySoundAtLocation` "/Game/Sounds/jump1.jump1" (0.0 0.0 0.0) (struct) 1.0 1.0 0.0 null null null)
          (`self.K2_SetActorRelativeLocation` (`KismetMathLibrary.MakeVector` _returnvalue_x (+ _returnvalue_y 150.0) _returnvalue_z))
          (`KismetSystemLibrary.Delay` 0.5)
          (set `self.BoolJump` false))))))

(event `InputAction|Backward`
  (params (Key :type "Key Structure"))
  (bind (_returnvalue_x _returnvalue_y _returnvalue_z) (`KismetMathLibrary.BreakVector` (`self.K2_GetActorLocation`)))
  ;[1 1 1] movement
  (:`Pressed`
    (if (not (`self.is Dead`))
      (bind _newparam (`self.isMovableBack`))
      (if _newparam
        (if (not (`self.BoolJump`))
          (`SceneComponent.K2_SetRelativeRotation` (`self.Mesh`) (struct :`Yaw` 180.0) false false)
          (`self.Jump`)
          (set `self.BoolJump` true)
          (`GameplayStatics.PlaySoundAtLocation` "/Game/Sounds/jump1.jump1" (0.0 0.0 0.0) (struct) 1.0 1.0 0.0 null null null)
          (`self.K2_SetActorRelativeLocation` (`KismetMathLibrary.MakeVector` (+ _returnvalue_x -150.0) _returnvalue_y _returnvalue_z))
          (`KismetSystemLibrary.Delay` 0.5)
          (set `self.BoolJump` false))))))

(event `InputAction|Forward`
  (params (Key :type "Key Structure"))
  (bind (_returnvalue_x _returnvalue_y _returnvalue_z) (`KismetMathLibrary.BreakVector` (`self.K2_GetActorLocation`)))
  ;[1 1 1] movement
  (:`Pressed`
    (if (`self.is Dead`)
      _
      (elif (not (`self.BoolJump`))
        (`SceneComponent.K2_SetRelativeRotation` :`self` (`self.Mesh`))
        (`self.Jump`)
        (set `self.BoolJump` true)
        (`GameplayStatics.PlaySoundAtLocation` "/Game/Sounds/jump1.jump1" (0.0 0.0 0.0) (struct) 1.0 1.0 0.0 null null null)
        (`self.K2_SetActorRelativeLocation` (`KismetMathLibrary.MakeVector` (+ _returnvalue_x 150.0) _returnvalue_y _returnvalue_z))
        (`KismetSystemLibrary.Delay` 0.5)
        (set `self.BoolJump` false)))))

(fn `ADDcoin`
  (set `self.coinvalue` (+ (`self.coinvalue`) 1))
  (`GameplayStatics.PlaySoundAtLocation` "/Game/Sounds/coin.coin" (0.0 0.0 0.0) (struct) 1.0 1.0 0.0 null null null))

(fn `Death`
  (bind _returnvalue (`self.K2_GetActorLocation`))
  (bind _returnvalue_2 (`self.K2_GetActorLocation`))
  (if (`self.traindeath`)
    (`self.DisableInput` null)
    (`GameplayStatics.PlaySoundAtLocation` "/Game/Sounds/smash.smash" (0.0 0.0 0.0) (struct) 1.0 1.0 0.0 null null null)
    (`SceneComponent.K2_SetWorldTransform` (`self.Mesh`) (`KismetMathLibrary.MakeTransform` (0.0 0.0 0.0) (struct) (1.5 1.5 0.1)) false false)
    (`GameplayStatics.SpawnEmitterAtLocation` "/Game/ParticleExplosions/Explode.Explode" _returnvalue_2)
    (`SceneComponent.ToggleVisibility` (`self.chicken`) false)
    (`GameplayStatics.SpawnEmitterAtLocation` "/Game/ParticleExplosions/Feather.Feather" _returnvalue_2)
    (elif (`self.waterdeath`)
      (`self.DisableInput` null)
      (`SceneComponent.K2_SetWorldTransform` (`self.Mesh`) (`KismetMathLibrary.MakeTransform` _returnvalue (struct) (1.5 1.5 0.1)) false false)
      (`GameplayStatics.PlaySoundAtLocation` "/Game/Sounds/chicken.chicken" (0.0 0.0 0.0) (struct) 1.0 1.0 0.0 null null null)
      (`SceneComponent.ToggleVisibility` (`self.chicken`) false)
      (`GameplayStatics.SpawnEmitterAtLocation` "/Game/ParticleExplosions/Drowning.Drowning" (`self.K2_GetActorLocation`))
      (else
        (`self.DisableInput` null)
        (`GameplayStatics.PlaySoundAtLocation` "/Game/Sounds/smash.smash" (0.0 0.0 0.0) (struct) 1.0 1.0 0.0 null null null)
        (`SceneComponent.K2_SetWorldTransform` (`self.Mesh`) (`KismetMathLibrary.MakeTransform` _returnvalue (struct) (1.5 1.5 0.1)) false false)
        (`GameplayStatics.SpawnEmitterAtLocation` "/Game/ParticleExplosions/Feather.Feather" _returnvalue)))))

(fn `hasfallen`
  (bind (_returnvalue_x _returnvalue_y _returnvalue_z) (`KismetMathLibrary.BreakVector` (`SceneComponent.K2_GetComponentLocation` (`self.chicken`))))
  (if (< _returnvalue_z 0.0)
    (set `self.is Dead` true)))

(fn `isMovableBack`
  (returns (NewParam :type Boolean))
  (bind _asmy_chicken (cast `/Game/BluePrints/MyChicken` (`GameplayStatics.GetPlayerPawn` 0)))
  (bind _returnvalue_x (`KismetMathLibrary.BreakVector` (`self.K2_GetActorLocation` _asmy_chicken)))
  (return (> (+ _returnvalue_x -150.0) -200.0)))

(fn `isMovableLeft`
  (returns (NewParam :type Boolean))
  (bind _asmy_chicken (cast `/Game/BluePrints/MyChicken` (`GameplayStatics.GetPlayerPawn` 0)))
  (bind (_returnvalue_x _returnvalue_y) (`KismetMathLibrary.BreakVector` (`self.K2_GetActorLocation` _asmy_chicken)))
  (return (> (+ _returnvalue_y -150.0) -1000.0)))

(fn `isMovableRIght`
  (returns (NewParam :type Boolean))
  (bind _asmy_chicken (cast `/Game/BluePrints/MyChicken` (`GameplayStatics.GetPlayerPawn` 0)))
  (bind (_returnvalue_x _returnvalue_y) (`KismetMathLibrary.BreakVector` (`self.K2_GetActorLocation` _asmy_chicken)))
  (return (< (+ _returnvalue_y 150.0) 1000.0)))

(fn `isObjectInWay`
  (returns (NewParam :type Boolean))
  (bind _astree (cast `/Game/Blueprints/tree` (`ActorComponent.GetOwner` (`self.Mesh`))))
  (bind _asmy_chicken (cast `/Game/BluePrints/MyChicken` (`GameplayStatics.GetPlayerPawn` 0)))
  (return (!= (`self.K2_GetActorLocation` _astree) (`self.K2_GetActorLocation` _asmy_chicken))))

(fn `restart`
  (if (`self.is Dead`)
    (`self.restart`)))

(fn `setscore`
  (bind _returnvalue_x (`KismetMathLibrary.BreakVector` (`CharacterMovementComponent.GetLastUpdateLocation` (`self.CharacterMovement`))))
  (if (> _returnvalue_x (+ (`self.scorelocation`) 100.0))
    (set `self.scorelocation` (+ (`self.scorelocation`) 100.0))
    (set `self.score` (+ (`self.score`) 50))))

(fn `UserConstructionScript`)