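; Game mode Blueprint that builds an initial stretch of randomly chosen floor tiles when play begins.
; BeginPlay repeatedly calls AddFloorTile, which spawns a random class from the FloorTiles array at NextSpawnPoint.
; Each spawned tile is cast to grass1, and its AttachTransform becomes the next spawn point, chaining tiles end to end.
; A failed cast leaves the spawn point unchanged.
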(event `self.ReceiveBeginPlay`
  (for _ (range 14)
    (`self.AddFloorTile`)))

(fn `AddFloorTile`
  (bind _floortiles (`self.FloorTiles`))
  (bind _returnvalue (`|SpawnActorFromClass` (`|GetArrayItem` _floortiles (`KismetMathLibrary.RandomIntegerInRange` 0 (`KismetArrayLibrary.Array_LastIndex` _floortiles))) (`self.NextSpawnPoint`) "Undefined" "OverrideRootScale" null null))
  (bind _asgrass_1 (cast `/Game/BluePrints/tiles/grass1` _returnvalue))
  (bind _newparam (`/Game/BluePrints/tiles/grass1.AttachTransform` _asgrass_1))
  (set `self.NextSpawnPoint` _newparam))

(fn `UserConstructionScript`)