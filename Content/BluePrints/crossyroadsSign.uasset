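; Sign actor, apparently for a Crossy Road-style game, that continuously bobs its static mesh up and down.
; On BeginPlay, two chained MoveComponentTo nodes raise and then lower the mesh along relative Z by Movedistance, one second each way.
; A single-iteration for loop wires back to the first move to repeat the cycle without Tick.
; Overlap, Tick and construction script are empty.
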(event `self.ReceiveBeginPlay`
  (bind _staticmesh (`self.StaticMesh`))
  (bind (_relativelocation_x _relativelocation_y _relativelocation_z) (`KismetMathLibrary.BreakVector` (`SceneComponent.RelativeLocation` _staticmesh)))
  (bind (_relativelocation_x_2 _relativelocation_y_2 _relativelocation_z_2) (`KismetMathLibrary.BreakVector` (`SceneComponent.RelativeLocation` (`self.StaticMesh`))))
  (`KismetSystemLibrary.MoveComponentTo` (`self.StaticMesh`) (`KismetMathLibrary.MakeVector` _relativelocation_x_2 _relativelocation_y_2 (+ _relativelocation_z_2 (`self.movedistance`))) (struct) false false 1.0 :!label _label)
  (`KismetSystemLibrary.MoveComponentTo` _staticmesh (`KismetMathLibrary.MakeVector` _relativelocation_x _relativelocation_y (- _relativelocation_z (`self.movedistance`))) (struct) false false 1.0)
  (for _ (range 1)
    (goto _label)))

(fn `UserConstructionScript`)