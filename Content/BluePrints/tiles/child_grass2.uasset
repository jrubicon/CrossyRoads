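; Grass tile Blueprint, a variant in the tiles set that scatters random child actors across itself.
; The construction script runs the parent's script, then Getspawns gathers the relative transforms of fourteen Randomspawn markers into Objectspawns.
; Spawnobject rolls one of eight branches per transform, each adding a child actor component at that spot.
; The event graph holds only disabled stubs, so all logic runs at construction.
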(fn `getspawns`
  (set `self.objectspawns` (`|MakeArray` (`SceneComponent.GetRelativeTransform` (`self.randomspawn1`)) (`SceneComponent.GetRelativeTransform` (`self.randomspawn2`)) (`SceneComponent.GetRelativeTransform` (`self.randomspawn3`)) (`SceneComponent.GetRelativeTransform` (`self.randomspawn4`)) (`SceneComponent.GetRelativeTransform` (`self.randomspawn5`)) (`SceneComponent.GetRelativeTransform` (`self.randomspawn6`)) (`SceneComponent.GetRelativeTransform` (`self.randomspawn7`)) (`SceneComponent.GetRelativeTransform` (`self.randomspawn8`)) (`SceneComponent.GetRelativeTransform` (`self.randomspawn9`)) (`SceneComponent.GetRelativeTransform` (`self.randomspawn10`)) (`SceneComponent.GetRelativeTransform` (`self.randomspawn11`)) (`SceneComponent.GetRelativeTransform` (`self.randomspawn13`)) (`SceneComponent.GetRelativeTransform` (`self.randomspawn14`)) (`SceneComponent.GetRelativeTransform` (`self.randomspawn12`)))))

(fn `Spawnobject`
  (for _array_element (`self.objectspawns`)
    (switch `int` (`KismetMathLibrary.RandomIntegerInRange` 0 7)
      (:`0`
        (`AddComponent|NODE_AddChildActorComponent-2` :`RelativeTransform` _array_element))
      (:`1`
        (`AddComponent|NODE_AddChildActorComponent-5` :`RelativeTransform` _array_element))
      (:`2`
        (`AddComponent|NODE_AddChildActorComponent-0` :`RelativeTransform` _array_element))
      (:`3`
        (`AddComponent|NODE_AddChildActorComponent-4` :`RelativeTransform` _array_element))
      (:`4`
        (`AddComponent|NODE_AddChildActorComponent-7` :`RelativeTransform` _array_element))
      (:`5`
        (`AddComponent|NODE_AddChildActorComponent-6` :`RelativeTransform` _array_element))
      (:`6`
        (`AddComponent|NODE_AddChildActorComponent-3` :`RelativeTransform` _array_element))
      (:`7`
        (`AddComponent|NODE_AddChildActorComponent-8` :`RelativeTransform` _array_element)))))

(fn `UserConstructionScript`
  (`parent.UserConstructionScript`)
  (`self.getspawns`)
  (`self.Spawnobject`))