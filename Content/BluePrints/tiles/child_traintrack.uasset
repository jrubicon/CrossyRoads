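; Train track tile, a child Blueprint that places a train at one of two spawn points on the tile.
; The construction script runs the parent's, then caches the relative transforms of Spawn and SpawnRight in the SpawnPoint array.
; A random coin flip then picks SpawnTrain or SpawnTrainRight, each adding a child actor component at its transform.
; BeginPlay and Tick only forward to the parent.
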(event `self.ReceiveBeginPlay`
  (`parent.ReceiveBeginPlay`))

(event `self.ReceiveTick`
  (params (DeltaSeconds :type "Float (single-precision)"))
  (`parent.ReceiveTick` DeltaSeconds))

(fn `setTrainSpawn`
  (set `self.SpawnPoint` (`|MakeArray` (`SceneComponent.GetRelativeTransform` (`self.Spawn`)) (`SceneComponent.GetRelativeTransform` (`self.SpawnRight`)))))

(fn `spawnTrain`
  (`AddComponent|NODE_AddChildActorComponent-1` :`RelativeTransform` (`|GetArrayItem` (`self.SpawnPoint`))))

(fn `spawnTrainRight`
  (`AddComponent|NODE_AddChildActorComponent-2` :`RelativeTransform` (`|GetArrayItem` (`self.SpawnPoint`) 1)))

(fn `UserConstructionScript`
  (`parent.UserConstructionScript`)
  (`self.setTrainSpawn`)
  (switch `int` (`KismetMathLibrary.RandomIntegerInRange` 0 1)
    (:`0`
      (`self.spawnTrain`))
    (:`1`
      (`self.spawnTrainRight`))))